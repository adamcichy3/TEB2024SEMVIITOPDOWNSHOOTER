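; Game mode for Mars Marine that spawns aliens continuously once play begins.
; After a short startup delay, it increments the wave counter once and starts a looping timer intended to fire the spawn-wave event by name.
; Each spawn-wave event places one BP_Alien at a random TargetPoint, drawn from every TargetPoint in the level.
; Nothing in this Blueprint stops the timer or advances to further waves.
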(event `self.ReceiveBeginPlay`
  (`KismetSystemLibrary.Delay` 2.0)
  (`self.StartNewWave`))

(event `Spawn Wave`
  (`self.SpawnAlien`))

(fn `GetRandomSpawnPoint`
  (returns (SpawnPoint :type "TargetPoint Object Reference"))
  (bind _outactors (`GameplayStatics.GetAllActorsOfClass` "/Script/Engine.TargetPoint"))
  (return (`|GetArrayItem` _outactors (`KismetMathLibrary.RandomIntegerInRange` 0 (`KismetArrayLibrary.Array_LastIndex` _outactors)))))

(fn `SpawnAlien`
  (bind _spawnpoint (`self.GetRandomSpawnPoint`))
  (`/Engine/EditorBlueprintResources/StandardMacros.IsValid` _spawnpoint
    (:`Is Valid`
      (`|SpawnActorFromClass` "/Game/Blueprints/AI/BP_Alien.BP_Alien_C" (`self.GetTransform` _spawnpoint) "Undefined" "OverrideRootScale" null null))))

(fn `StartNewWave`
  (`/Engine/EditorBlueprintResources/StandardMacros.IncrementInt` (`self.CurrentWave`)
    (:`  `
      (`KismetSystemLibrary.K2_SetTimer` null "Spawn Wave" 5.0 true))))

(fn `UserConstructionScript`)